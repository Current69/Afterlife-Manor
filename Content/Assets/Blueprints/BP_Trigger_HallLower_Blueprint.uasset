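; Trigger volume for the lower hall that reports the player's room and drives a journal update.
; When a player-controlled pawn overlaps the Box, it passes RoomType to the BP_Character_Pawn's UpdatePlayerLocation on every entry.
; It also sends JournalEntry to that pawn's JournalManager until UpdateChecker returns true, which is stored in JournalTriggered to block further updates.
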(event OnComponentBeginOverlap(Box)
  (params (OverlappedComponent :type Primitive%20Component%20Object%20Reference) (OtherActor :type Actor%20Object%20Reference) (OtherComp :type Primitive%20Component%20Object%20Reference) (OtherBodyIndex :type Integer) (bFromSweep :type Boolean) (SweepResult :type Hit%20Result%20Structure%20%28by%20ref%29))
  (if (Pawn|IsPlayerControlled (Variables|/Script/Engine.Actor|GetInstigator OtherActor))
    (bind _asbp_character_pawn (Utilities|Casting|CastToBP_Character_Pawn OtherActor))
    (Default|UpdatePlayerLocation _asbp_character_pawn (Variables|Default|GetRoomType))
    (if (not (Variables|Default|GetJournal%20Triggered))
      (Default|JournalUpdate (Variables|/Game/Assets/Blueprints/BP_Character_Pawn.BP_Character_Pawn_C|GetJournal%20Manager _asbp_character_pawn) (Variables|Default|GetJournal%20Entry))
      (bind _newparam1 (Default|UpdateChecker (Variables|/Game/Assets/Blueprints/BP_Character_Pawn.BP_Character_Pawn_C|GetJournal%20Manager _asbp_character_pawn)))
      (Variables|Default|SetJournal%20Triggered _newparam1))))

(event EventBeginPlay
  (|CallParentFunction) ; This node is disabled and will not be called.\nDrag off pins to build functionality.
)

(event Collision|EventActorBeginOverlap
  (params (OtherActor :type Actor%20Object%20Reference))
  (|CallParentFunction OtherActor) ; This node is disabled and will not be called.\nDrag off pins to build functionality.
)

(event EventTick
  (params (DeltaSeconds :type Float%20%28single-precision%29))
  (|CallParentFunction DeltaSeconds) ; This node is disabled and will not be called.\nDrag off pins to build functionality.
)

(fn ConstructionScript
  (|CallParentFunction))