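; Player character with axis-driven movement and look, using camera vectors for movement when a head-mounted display is enabled.
; Left click traces under the cursor for nearby pickup objects, stores their type and image, updates the pause menu inventory, then destroys them.
; M toggles the pause menu widget and game pause.
; The menu's pain level flags set walk speed and gate Shift sprinting, which doubles speed until release reapplies the pain level.
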(event Custom|SetPainLevel
  (bind _charactermovement (Variables|Character|GetCharacterMovement))
  (bind _pausemenureference (Variables|Default|GetPauseMenuReference))
  ;[1 1 1] SetPlayerSpeed
  (if (Variables|/Game/Assets/Blueprints/BP_PauseMenuHUD.BP_PauseMenuHUD_C|GetPain%20Level%200 _pausemenureference)
    (Variables|/Script/Engine.CharacterMovementComponent|SetMaxWalkSpeed _charactermovement 1e+02)
    (Variables|Default|SetCanSprint false :!label _label)
    (elif (Variables|/Game/Assets/Blueprints/BP_PauseMenuHUD.BP_PauseMenuHUD_C|GetPain%20Level%201 _pausemenureference)
      (Variables|/Script/Engine.CharacterMovementComponent|SetMaxWalkSpeed _charactermovement 2e+02)
      (goto _label)
      (else
        (Variables|/Script/Engine.CharacterMovementComponent|SetMaxWalkSpeed _charactermovement 3e+02)
        (Variables|Default|SetCanSprint true)))))

(event EventBeginPlay
  ;[1 1 1] GetPlayerHUD
  (bind _returnvalue (UserInterface|CreateWidget "/Game/Assets/Blueprints/BP_PlayerHUD.BP_PlayerHUD_C"))
  (UserInterface|Viewport|AddtoViewport _returnvalue 0)
  (Variables|/Script/Engine.CharacterMovementComponent|SetMaxWalkSpeed (Variables|Character|GetCharacterMovement) 3e+02)
  (bind _returnvalue_2 (UserInterface|CreateWidget "/Game/Assets/Blueprints/BP_PauseMenuHUD.BP_PauseMenuHUD_C"))
  (Variables|Default|SetPauseMenuReference _returnvalue_2))

(event EventTick
  (params (DeltaSeconds :type Float%20%28single-precision%29)))

(event Collision|EventActorBeginOverlap
  (params (OtherActor :type Actor%20Object%20Reference)))

(event Input|AxisEvents|InputAxisMoveForward
  (params (AxisValue :type Float%20%28single-precision%29))
  ;[1 1 1] Movement Controls
  (Pawn|Input|AddMovementInput (select (Class|HeadMountedDisplayFunctionLibrary|IsHeadMountedDisplayEnabled) (Math|Vector|GetForwardVector (Variables|Default|GetCamera)) (Transformation|GetActorForwardVector)) AxisValue false))

(event Input|AxisEvents|InputAxisMoveSide
  (params (AxisValue :type Float%20%28single-precision%29))
  ;[1 1 1] Movement Controls
  (Pawn|Input|AddMovementInput (select (Class|HeadMountedDisplayFunctionLibrary|IsHeadMountedDisplayEnabled) (Math|Vector|GetRightVector (Variables|Default|GetCamera)) (Transformation|GetActorRightVector)) AxisValue false))

(event Input|AxisEvents|InputAxisTurn
  (params (AxisValue :type Float%20%28single-precision%29))
  ;[1 1 1] Movement Controls
  (Pawn|Input|AddControllerYawInput AxisValue))

(event Input|AxisEvents|InputAxisLookUp
  (params (AxisValue :type Float%20%28single-precision%29))
  ;[1 1 1] Movement Controls
  (Pawn|Input|AddControllerPitchInput AxisValue))

(event Input|KeyboardEvents|M
  (params (Key :type Key%20Structure :default "None"))
  (bind _returnvalue (Game|GetPlayerController 0))
  ;[1 1 1] Pause/Unpause
  (:Pressed
    (if (Game|IsGamePaused)
      (Variables|/Script/Engine.PlayerController|SetbShowMouseCursor _returnvalue false)
      (Widget|RemovefromParent (Variables|Default|GetPauseMenuReference))
      (Game|SetGamePaused false)
      (else
        (Utilities|IsValid (Variables|Default|GetPauseMenuReference)
          (:Is%20Valid
            _)
          (:Is%20Not%20Valid
            (bind _returnvalue_2 (UserInterface|CreateWidget "/Game/Assets/Blueprints/BP_PauseMenuHUD.BP_PauseMenuHUD_C"))
            (Variables|Default|SetPauseMenuReference _returnvalue_2)))
        (Variables|/Script/Engine.PlayerController|SetbShowMouseCursor _returnvalue true)
        (UserInterface|Viewport|AddtoViewport (Variables|Default|GetPauseMenuReference) 0)
        (Game|SetGamePaused true)))))

(event Input|MouseEvents|LeftMouseButton
  (params (Key :type Key%20Structure :default "None"))
  (bind _returnvalue (Game|GetPlayerController 0))
  (bind _array (Utilities|Array|MakeArray "ObjectTypeQuery7"))
  (bind _hitresult (Class|PlayerController|GetHitResultUnderCursorforObjects _returnvalue _array true))
  (bind (_bblockinghit _binitialoverlap _time _distance _location _impactpoint _normal _impactnormal _physmat _hitactor) (Collision|BreakHitResult _hitresult))
  ;[1 1 1] PickUpObject
  (:Pressed
    (if _bblockinghit
      (Math|Float|CompareFloat (Transformation|GetDistanceTo (Game|GetPlayerCharacter 0) _hitactor) 2e+02
        (:<
          (bind _asbp_master_pickup_object (Utilities|Casting|CastToBP_Master_Pickup_Object _hitactor))
          (Utilities|Map|Add (Variables|Default|GetPlayerInventory) (Variables|/Game/Assets/Objects/Master_Blueprints/BP_Master_Pickup_Object.BP_Master_Pickup_Object_C|GetPickUpType _asbp_master_pickup_object) true)
          (Utilities|Map|Add (Variables|Default|GetInventoryPictures) (Variables|/Game/Assets/Objects/Master_Blueprints/BP_Master_Pickup_Object.BP_Master_Pickup_Object_C|GetPickUpType _asbp_master_pickup_object) (Variables|/Game/Assets/Objects/Master_Blueprints/BP_Master_Pickup_Object.BP_Master_Pickup_Object_C|GetItemImage _asbp_master_pickup_object))
          (Default|UpdateInventory (Variables|Default|GetPauseMenuReference) (Variables|/Game/Assets/Objects/Master_Blueprints/BP_Master_Pickup_Object.BP_Master_Pickup_Object_C|GetPickUpType _asbp_master_pickup_object))
          (Actor|DestroyActor _hitactor))))))

(event Input|KeyboardEvents|LeftShift
  (params (Key :type Key%20Structure :default "None"))
  (bind _charactermovement (Variables|Character|GetCharacterMovement))
  ;[1 1 1] Sprint
  (:Pressed
    (if (Variables|Default|GetCanSprint)
      (Variables|/Script/Engine.CharacterMovementComponent|SetMaxWalkSpeed _charactermovement (* (Variables|/Script/Engine.CharacterMovementComponent|GetMaxWalkSpeed (Variables|Character|GetCharacterMovement)) 2.0))))
  (:Released
    (Variables|/Script/Engine.CharacterMovementComponent|SetMaxWalkSpeed _charactermovement (Variables|/Script/Engine.CharacterMovementComponent|GetMaxWalkSpeed (Variables|Character|GetCharacterMovement)))
    (CallFunction|SetPainLevel)))

(fn ConstructionScript)