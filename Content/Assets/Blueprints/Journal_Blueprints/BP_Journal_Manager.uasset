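; BP_Journal_Manager is an actor that tracks journal progress through a referenced TestJournal object.
; The JournalUpdate event switches on the incoming JournalEntry and increments TestJournal's JournalProgress when that reference is valid.
; UpdateChecker reports whether that progress is above zero, again guarded by a validity check.
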(event Custom|Journal%20Update
  (params (Journal%20Entry :type E_Journals%20Enum :default "NewEnumerator0"))
  (bind _test_journal (Variables|Default|GetTest%20Journal))
  (switch Utilities|FlowControl|Switch|SwitchonE_Journals Journal%20Entry
    (:NewEnumerator0
      (Utilities|IsValid _test_journal
        (:Is%20Valid
          (Variables|/Game/Assets/Blueprints/HUD_Blueprints/Journals/BP_HUD_TestJournal.BP_HUD_TestJournal_C|SetJournal%20Progress _test_journal (+ (Variables|/Game/Assets/Blueprints/HUD_Blueprints/Journals/BP_HUD_TestJournal.BP_HUD_TestJournal_C|GetJournal%20Progress _test_journal) 1)))))))

(event EventBeginPlay)

(event Collision|EventActorBeginOverlap
  (params (OtherActor :type Actor%20Object%20Reference)))

(event EventTick
  (params (DeltaSeconds :type Float%20%28single-precision%29)))

(fn ConstructionScript)

(fn UpdateChecker
  (bind _test_journal (Variables|Default|GetTest%20Journal))
  (Utilities|IsValid _test_journal
    (:Is%20Valid
      (return (> (Variables|/Game/Assets/Blueprints/HUD_Blueprints/Journals/BP_HUD_TestJournal.BP_HUD_TestJournal_C|GetJournal%20Progress _test_journal) 0)))))