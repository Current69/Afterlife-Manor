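; Interactable darkness shrine with a candle that takes item offerings to raise the player's sight level, capped at 3.
; Interacting either uses an item on the shrine or hits the candle, which lights only if the player has matches.
; Lighting it with a held item accepts or declines the offering; acceptance below the cap updates the GameInstance darkness level and displays the item.
; A looping-style timeline drives candle light flicker.
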(event Custom|Event%20CandleHit
  ;[1 1 1] On Candle Hit
  (Utilities|IsValid (Variables|Default|GetPlayerBlueprint)
    (:Is%20Valid
      _)
    (:Is%20Not%20Valid
      (bind _asbp_character_pawn (Utilities|Casting|CastToBP_Character_Pawn (Game|GetPlayerCharacter 0)))
      (Variables|Default|SetPlayerBlueprint _asbp_character_pawn)))
  (if (Variables|/Game/Assets/Blueprints/BP_Character_Pawn.BP_Character_Pawn_C|GetHasMatches (Variables|Default|GetPlayerBlueprint))
    (Development|PrintString "Has the Matches, Begin Fire Effect")
    (CallFunction|SetEnabled true)
    (if (Variables|Default|GetItemHeld)
      (if (Variables|Default|GetHeldItemAcceptable)
        (CallFunction|ShrineAccepts)
        (else
          (CallFunction|ShrineDeclines))))
    (else
      (Development|PrintString "No matches, no fire effect")
      (CallFunction|SetEnabled false)))
  (Variables|Default|SetCandleClicked false))

(event EventBeginPlay
  ;[1 1 1] Begin Play Setup
  (Collision|SetCollisionObjectType (Variables|Default|GetCube) "ECC_GameTraceChannel2")
  (Collision|SetCollisionObjectType (Variables|Default|GetCandle) "ECC_GameTraceChannel3")
  (bind _intensity (Timeline|CandleFlickerTimeline Play)
    (:Update
      (Rendering|Components|Light|SetIntensity (Variables|Default|GetPointLight) (Math|Float|Lerp (Variables|Default|GetMinIntensity) (Variables|Default|GetMaxIntensity) _intensity)))))

(event Collision|EventActorBeginOverlap
  (params (OtherActor :type Actor%20Object%20Reference))
  (|CallParentFunction OtherActor) ; This node is disabled and will not be called.\nDrag off pins to build functionality.
)

(event EventTick
  (params (DeltaSeconds :type Float%20%28single-precision%29))
  (|CallParentFunction DeltaSeconds) ; This node is disabled and will not be called.\nDrag off pins to build functionality.
)

(event EventShrineAccepts
  ;[1 1 1] Shrine Accepts
  (Development|PrintString "Your Offering is Acceptable")
  (bind _asbp_level_transfer (Utilities|Casting|CastToBP_LevelTransfer (Game|GetGameInstance)))
  (Math|Integer|CompareInt (Variables|/Game/Assets/Blueprints/BP_LevelTransfer.BP_LevelTransfer_C|GetCurrent%20Sight%20Level _asbp_level_transfer) 3
    (:<
      (Default|UpdateDarknessLevel _asbp_level_transfer (+ (Variables|/Game/Assets/Blueprints/BP_LevelTransfer.BP_LevelTransfer_C|GetCurrent%20Sight%20Level _asbp_level_transfer) 1))
      (CallFunction|DisplayItem))))

(event EventShrineInteract
  ;[1 1 1] Shrine Interact
  (if (Variables|Default|GetCandleClicked)
    (CallFunction|EventCandleHit)
    (else
      (CallFunction|UseItem self))))

(fn ConstructionScript
  (|CallParentFunction)
  (CallFunction|SetEnabled (Variables|Default|GetEnabled)))

(fn SetEnabled
  (params (Enabled :type Boolean))
  (bind _output_get (Variables|Default|SetEnabled Enabled))
  (Rendering|SetVisibility (Variables|Default|GetPointLight) _output_get false)
  (Rendering|SetVisibility (Variables|Default|GetFireEffect) _output_get false)
  (Rendering|SetCastShadow (Variables|Default|GetCandle) (not _output_get)))