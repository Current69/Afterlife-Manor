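; BP_Door_Master is a door Blueprint, apparently a master for door objects, that swings open and closed through the DoorIntereact event.
; The event plays or reverses a timeline based on the Open flag, lerping the door's relative yaw between ClosePos and OpenPos and flipping Open on finish.
; Play rate comes from the inverse of a duration, with TimeToClose used when opening and TimeToOpen when closing.
; BeginPlay assigns the door a custom collision object type.
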(event Custom|Door%20Intereact
  (bind _opendoortimeline (Variables|Default|GetOpenDoorTimeline))
  (if (Variables|Default|GetOpen)
    (Development|PrintString "Door close")
    (Components|Timeline|SetPlayRate _opendoortimeline (/ 1.0 (Variables|Default|GetTimeToOpen)))
    (bind _doortrack (Timeline|OpenDoorTimeline Reverse)
      (:Update
        (Transformation|SetRelativeRotation (Variables|Default|GetDoor) (Math|Rotator|MakeRotator 0.0 0.0 (Math|Float|Lerp (Variables|Default|GetClosePos) (Variables|Default|GetOpenPos) _doortrack)) false false))
      (:Finished
        (Variables|Default|SetOpen (not (Variables|Default|GetOpen)))))
    (else
      (Development|PrintString "Door open")
      (Components|Timeline|SetPlayRate _opendoortimeline (/ 1.0 (Variables|Default|GetTimeToClose)))
      (Timeline|OpenDoorTimeline Play))))

(event EventBeginPlay
  (Collision|SetCollisionObjectType (Variables|Default|GetDoor) "ECC_GameTraceChannel2"))

(event Collision|EventActorBeginOverlap
  (params (OtherActor :type Actor%20Object%20Reference)))

(event EventTick
  (params (DeltaSeconds :type Float%20%28single-precision%29)))

(fn ConstructionScript)