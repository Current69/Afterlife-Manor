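; BP_Slide_Door is a sliding door with open, close and locked-shake events, plus a pausing use-item menu.
; One timeline slides the door forward or in reverse at rates from open/close times, while another shakes it when it stays locked.
; UnlockSide and UnblockSide overlap volumes track which side the player occupies.
; UseItem toggles BP_UseItemHUD, passing it the interacting shrine and door on creation.
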(event OnComponentBeginOverlap(UnblockSide)
  (params (OverlappedComponent :type Primitive%20Component%20Object%20Reference) (OtherActor :type Actor%20Object%20Reference) (OtherComp :type Primitive%20Component%20Object%20Reference) (OtherBodyIndex :type Integer) (bFromSweep :type Boolean) (SweepResult :type Hit%20Result%20Structure%20%28by%20ref%29))
  ;[1 1 1] Unblock Area
  (Utilities|IsValid OtherActor
    (:Is%20Valid
      (Variables|Default|SetPlayerInUnblockArea (== OtherActor (Game|GetPlayerCharacter 0))))))

(event OnComponentEndOverlap(UnblockSide)
  (params (OverlappedComponent :type Primitive%20Component%20Object%20Reference) (OtherActor :type Actor%20Object%20Reference) (OtherComp :type Primitive%20Component%20Object%20Reference) (OtherBodyIndex :type Integer))
  ;[1 1 1] Unblock Area
  (Utilities|IsValid OtherActor
    (:Is%20Valid
      (Variables|Default|SetPlayerInUnblockArea (not (== OtherActor (Game|GetPlayerCharacter 0)))))))

(event OnComponentBeginOverlap(UnlockSide)
  (params (OverlappedComponent :type Primitive%20Component%20Object%20Reference) (OtherActor :type Actor%20Object%20Reference) (OtherComp :type Primitive%20Component%20Object%20Reference) (OtherBodyIndex :type Integer) (bFromSweep :type Boolean) (SweepResult :type Hit%20Result%20Structure%20%28by%20ref%29))
  ;[1 1 1] Unlock Side
  (Utilities|IsValid OtherActor
    (:Is%20Valid
      (Variables|Default|SetPlayerInUnlockArea (== OtherActor (Game|GetPlayerCharacter 0))))))

(event OnComponentEndOverlap(UnlockSide)
  (params (OverlappedComponent :type Primitive%20Component%20Object%20Reference) (OtherActor :type Actor%20Object%20Reference) (OtherComp :type Primitive%20Component%20Object%20Reference) (OtherBodyIndex :type Integer))
  ;[1 1 1] Unlock Side
  (Utilities|IsValid OtherActor
    (:Is%20Valid
      (Variables|Default|SetPlayerInUnlockArea (not (== OtherActor (Game|GetPlayerCharacter 0)))))))

(event EventBeginPlay
  (|CallParentFunction) ; This node is disabled and will not be called.\nDrag off pins to build functionality.
)

(event Collision|EventActorBeginOverlap
  (params (OtherActor :type Actor%20Object%20Reference))
  (|CallParentFunction OtherActor) ; This node is disabled and will not be called.\nDrag off pins to build functionality.
)

(event EventTick
  (params (DeltaSeconds :type Float%20%28single-precision%29))
  (|CallParentFunction DeltaSeconds) ; This node is disabled and will not be called.\nDrag off pins to build functionality.
)

(event EventDoorClose
  ;[1 1 1] Door Interaction
  (Variables|Default|SetDoorInMotion true)
  (if (== (Variables|Default|GetOpen) (Variables|Default|GetLast%20Setting))
    (Audio|PlaySoundatLocation "/Game/Sounds/Door_Sliding_Close_1.Door_Sliding_Close_1" "0, 0, 0" "0, 0, 0" 1.0 1.0 0.0 0 0 0 0))
  (Development|PrintString "Door close")
  (Variables|Default|SetOpen false)
  (Components|Timeline|SetPlayRate (Variables|Default|GetSlide%20Door%20Timeline) (/ 1.0 (Variables|Default|GetTimeToClose)))
  (bind _doortrack (Timeline|Slide%20Door%20Timeline Reverse)
    (:Update
      (Transformation|SetRelativeTransform (Variables|Default|GetDoor) (Math|Transform|MakeTransform (Math|Vector|MakeVector (Math|Float|Lerp (Variables|Default|GetClosePos) (Variables|Default|GetOpenPos) _doortrack) 0.0 0.0) "0, 0, 0" "1.000000,1.000000,1.000000") false false))
    (:Finished
      (Variables|Default|SetLast%20Setting (Variables|Default|GetOpen))
      (Variables|Default|SetDoorInMotion false))))

(event EventDoorOpen
  ;[1 1 1] Door Interaction
  (Variables|Default|SetDoorInMotion true)
  (if (== (Variables|Default|GetOpen) (Variables|Default|GetLast%20Setting))
    (Audio|PlaySoundatLocation "/Game/Sounds/Door_Sliding_Open_1.Door_Sliding_Open_1" "0, 0, 0" "0, 0, 0" 1.0 1.0 0.0 0 0 0 0))
  (Development|PrintString "Door open")
  (Variables|Default|SetOpen true)
  (Components|Timeline|SetPlayRate (Variables|Default|GetSlide%20Door%20Timeline) (/ 1.0 (Variables|Default|GetTimeToOpen)))
  (bind _doortrack (Timeline|Slide%20Door%20Timeline Play)
    (:Update
      (Transformation|SetRelativeTransform (Variables|Default|GetDoor) (Math|Transform|MakeTransform (Math|Vector|MakeVector (Math|Float|Lerp (Variables|Default|GetClosePos) (Variables|Default|GetOpenPos) _doortrack) 0.0 0.0) "0, 0, 0" "1.000000,1.000000,1.000000") false false))
    (:Finished
      (Variables|Default|SetLast%20Setting (Variables|Default|GetOpen))
      (Variables|Default|SetDoorInMotion false))))

(event EventDoorStaysLocked
  ;[1 1 1] Door Interaction
  (Variables|Default|SetDoorInMotion true)
  (bind _doortrack (Timeline|Shake%20Door%20Timeline PlayFromStart)
    (:Update
      (Transformation|SetRelativeTransform (Variables|Default|GetDoor) (Math|Transform|MakeTransform (Math|Vector|MakeVector (Math|Float|Lerp 0.0 2.5 _doortrack) 0.0 0.0) "0, 0, 0" "1.000000,1.000000,1.000000") false false))
    (:Finished
      (Development|PrintString "Door is locked from this side")
      (Variables|Default|SetDoorInMotion false))))

(event EventUseItem
  (params (Interacting%20Shrine :type BP%20Master%20Shrine%20Object%20Reference) (Interacting%20Door :type BP%20Door%20Master%20Object%20Reference))
  (bind _returnvalue (Game|GetPlayerController 0))
  ;[1 1 1] Spawn Use Menu
  (if (Game|IsGamePaused)
    (Variables|/Script/Engine.PlayerController|SetbShowMouseCursor _returnvalue false)
    (Input|SetInputModeGameOnly _returnvalue)
    (Widget|RemovefromParent (Variables|Default|GetUse%20Item%20Menu))
    (Game|SetGamePaused false)
    (else
      (Utilities|IsValid (Variables|Default|GetUse%20Item%20Menu)
        (:Is%20Valid
          _)
        (:Is%20Not%20Valid
          (bind _returnvalue_2 (UserInterface|CreateWidget "/Game/Assets/Blueprints/HUD_Blueprints/BP_UseItemHUD.BP_UseItemHUD_C"))
          (Variables|Default|SetUse%20Item%20Menu _returnvalue_2)
          (Variables|/Game/Assets/Blueprints/HUD_Blueprints/BP_UseItemHUD.BP_UseItemHUD_C|SetInteracting%20Shrine _returnvalue_2 Interacting%20Shrine)
          (Variables|/Game/Assets/Blueprints/HUD_Blueprints/BP_UseItemHUD.BP_UseItemHUD_C|SetInteracting%20Door _returnvalue_2 Interacting%20Door)))
      (Variables|/Script/Engine.PlayerController|SetbShowMouseCursor _returnvalue true)
      (UserInterface|Viewport|AddtoViewport (Variables|Default|GetUse%20Item%20Menu) 0)
      (Game|SetGamePaused true))))

(fn ConstructionScript
  (|CallParentFunction))