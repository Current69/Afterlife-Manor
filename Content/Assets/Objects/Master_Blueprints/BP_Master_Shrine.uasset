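; Master shrine actor that opens an item-offering menu when interacted with.
; ShrineInteract calls UseItem, which toggles a cached BP_UseItemHUD widget along with game pause and mouse cursor, passing shrine and door references when first created.
; ShrineAccepts and ShrineDeclines only print feedback messages.
; BeginPlay assigns the Cube a custom collision object type.
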(event Custom|Shrine%20Accepts
  (Development|PrintString "Your Offering is Acceptable"))

(event Custom|Shrine%20Interact
  (CallFunction|UseItem self))

(event Custom|Shrine%20Declines
  (Development|PrintString "Your offering is bad and you should feel bad"))

(event Custom|Use%20Item
  (params (Interacting%20Shrine :type BP%20Master%20Shrine%20Object%20Reference) (Interacting%20Door :type BP%20Door%20Master%20Object%20Reference))
  (bind _returnvalue (Game|GetPlayerController 0))
  ;[1 1 1] Spawn Use Menu
  (if (Game|IsGamePaused)
    (Variables|/Script/Engine.PlayerController|SetbShowMouseCursor _returnvalue false)
    (Input|SetInputModeGameOnly _returnvalue)
    (Widget|RemovefromParent (Variables|Default|GetUse%20Item%20Ref))
    (Game|SetGamePaused false)
    (else
      (Utilities|IsValid (Variables|Default|GetUse%20Item%20Ref)
        (:Is%20Valid
          _)
        (:Is%20Not%20Valid
          (bind _returnvalue_2 (UserInterface|CreateWidget "/Game/Assets/Blueprints/HUD_Blueprints/BP_UseItemHUD.BP_UseItemHUD_C"))
          (Variables|Default|SetUse%20Item%20Ref _returnvalue_2)
          (Variables|/Game/Assets/Blueprints/HUD_Blueprints/BP_UseItemHUD.BP_UseItemHUD_C|SetInteracting%20Shrine _returnvalue_2 Interacting%20Shrine)
          (Variables|/Game/Assets/Blueprints/HUD_Blueprints/BP_UseItemHUD.BP_UseItemHUD_C|SetInteracting%20Door _returnvalue_2 Interacting%20Door)))
      (Variables|/Script/Engine.PlayerController|SetbShowMouseCursor _returnvalue true)
      (UserInterface|Viewport|AddtoViewport (Variables|Default|GetUse%20Item%20Ref) 0)
      (Game|SetGamePaused true))))

(event EventBeginPlay
  (Collision|SetCollisionObjectType (Variables|Default|GetCube) "ECC_GameTraceChannel2"))

(event Collision|EventActorBeginOverlap
  (params (OtherActor :type Actor%20Object%20Reference)))

(event EventTick
  (params (DeltaSeconds :type Float%20%28single-precision%29)))

(fn ConstructionScript)