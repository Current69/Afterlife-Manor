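; BP_Master_PointLight is a master point light Blueprint whose intensity and color change with a sight level.
; UpdateLightLevel and UpdateLightColor clamp the given level to one of three steps and use it to index the SightLevels and NewLightColor arrays, applying the result to the point light component.
; BeginPlay caches the starting color in DefaultLightColor, which nothing in these graphs reads back.
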(event EventBeginPlay
  (Variables|Default|SetDefault%20Light%20Color (Rendering|Components|Light|GetLightColor (Variables|Default|GetLightComponent))))

(event EventTick
  (params (DeltaSeconds :type Float%20%28single-precision%29)))

(fn ConstructionScript)

(fn UpdateLightLevel
  (params (CurrentSightLevel :type Integer))
  (Rendering|Components|Light|SetIntensity (Variables|Default|GetPointLightComponent) (Utilities|Array|Get(acopy) (Variables|Default|GetSightLevels) (Math|Integer|Clamp(Integer) CurrentSightLevel 0 2))))

(fn UpdateLightColor
  (params (CurrentSightLevel :type Integer))
  (Rendering|Components|Light|SetLightColor (Variables|Default|GetPointLightComponent) (Utilities|Array|Get(acopy) (Variables|Default|GetNew%20Light%20Color) (Math|Integer|Clamp(Integer) CurrentSightLevel 0 2)) true))